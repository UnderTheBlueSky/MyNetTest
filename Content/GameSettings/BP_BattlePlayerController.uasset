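; Player controller for battle matches that drives match UI and end-of-game screens for the local player.
; It adds player entries to a list widget, has the controlled battle character set up other players' UI, and forwards wait/ready states to the Level Blueprint via "ce" console commands.
; Win and lose events clear all widgets and the character's sprint and health timers, then show the matching result widget.
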(event Custom|CreatePlayerInfo
  (params (PlayerState :type Battle%20Player%20State%20Object%20Reference))
  ;[1 1 1] 创建一个玩家的信息
  (bind _asplayer_list (Utilities|Casting|CastToPlayerList (Variables|Default|GetPlayerListWidget)))
  (Default|AddPlayer _asplayer_list PlayerState))

(event Custom|WaitToStart
  ;[1 1 1] 调用关卡蓝图事件
  (Development|ExecuteConsoleCommand "ce ShowWaitUI" 0))

(event Custom|ReadyPlay
  ;[1 1 1] 调用关卡蓝图事件
  (Development|ExecuteConsoleCommand "ce ReadyPlay" 0))

(event Custom|ShowOtherPlayerUI
  ;[1 1 1] 显示其他玩家UI
  (bind _asbp_battle_character (Utilities|Casting|CastToBP_BattleCharacter (Pawn|GetControlledPawn)))
  (Default|InitPlayers _asbp_battle_character))

(event Custom|GameWin
  ;[1 1 1] 游戏结束
  (CallFunction|ClearTimerandWidget)
  (bind _returnvalue (UserInterface|CreateWidget "/Game/UI/WinnerUI.WinnerUI_C" self))
  (UserInterface|Viewport|AddtoViewport _returnvalue 0))

(event Custom|ClearTimerAndWidget
  ;[1 1 1] 游戏结束
  (Viewport|RemoveAllWidgets)
  (bind _asbp_battle_character (Utilities|Casting|CastToBP_BattleCharacter (Pawn|GetControlledPawn)))
  (Utilities|Time|ClearandInvalidateTimerbyHandle (Variables|/Script/MyNetTest.BattleCharacter|GetMySprintTimerHandle _asbp_battle_character))
  (Utilities|Time|ClearandInvalidateTimerbyHandle (Variables|/Script/MyNetTest.BattleCharacter|GetHealthTimerHandle _asbp_battle_character)))

(event Custom|GameLose
  ;[1 1 1] 游戏结束
  (CallFunction|ClearTimerandWidget)
  (bind _returnvalue (UserInterface|CreateWidget "/Game/UI/GameLose.GameLose_C"))
  (UserInterface|Viewport|AddtoViewport _returnvalue 0))

(fn ConstructionScript)