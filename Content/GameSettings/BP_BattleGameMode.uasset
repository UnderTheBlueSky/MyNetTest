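; Battle game mode that runs a multiplayer match from player login through win or loss.
; PostLogin holds players waiting until the GameInstance's player limit is reached, then readies every controller.
; A looping timer spawns trigger actors at random navigable points.
; Deaths leave player-colored death actors; the last survivor or first player reaching full health wins, clearing triggers and notifying each controller of the result.
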(event Custom|Deal%20with%20players
  (params (Character :type Pawn%20Object%20Reference))
  ;[1 1 1] 游戏结束，每个玩家的处理
  (for _array_element (Variables|Default|GetPlayerControllerList)
    (Utilities|IsValid _array_element
      (:Is%20Valid
        (if (== (Pawn|GetController Character) _array_element)
          (Default|GameWin _array_element)
          (else
            (Default|GameLose _array_element)))))))

(event Custom|ShowAllPlayerUI
  ;[1 1 1] ShowAllPlayerUI
  (for _array_element (Variables|Default|GetPlayerControllerList)
    (Default|ShowOtherPlayerUI _array_element)))

(event Custom|DestoryAllTriggerActor
  ;[1 1 1] 游戏结束时 删除所有的TriggerActor
  (bind _outactors (Actor|GetAllActorsOfClass "/Game/TriggerActor/BP_TriggerActor.BP_TriggerActor_C"))
  (for _array_element _outactors
    (Actor|DestroyActor _array_element))
  (Utilities|Time|ClearandInvalidateTimerbyHandle (Variables|Default|GetSpawnTriggerActorHandle)))

(event Custom|SpawnTriggerActorToRandomLocation
  ;[1 1 1] SpawnTriggerActor
  (bind _returnvalue (Utilities|Time|SetTimerbyEvent (delegate Custom|SpawnTriggerActor) 2.0 true))
  (Variables|Default|SetSpawnTriggerActorHandle _returnvalue))

(event Custom|SpawnTriggerActor
  ;[1 1 1] SpawnTriggerActor
  (bind _randomlocation (Class|NavigationSystemV1|GetRandomLocationinNavigableRadius (Variables|Default|GetOriginLocation) (Variables|Default|GetRedius) 0 0))
  (Game|SpawnActorfromClass (Variables|Default|GetTriggerActorClass) (Math|Conversions|ToTransform(Vector) _randomlocation) "AlwaysSpawn" 0 0))

(event EventPlayerPawnDeath
  (params (Character :type Battle%20Character%20Object%20Reference))
  ;[1 1 1] 有玩家死亡时的事件
  (bind _asbattle_player_state (Utilities|Casting|CastToBattlePlayerState (Variables|/Script/Engine.Pawn|GetPlayerState Character)))
  (bind _returnvalue (Game|SpawnActorfromClass "/Game/Character/BP_DeathActor.BP_DeathActor_C" (Transformation|GetWorldTransform (Variables|/Script/Engine.Character|GetMesh Character)) "AlwaysSpawn" 0 (Variables|/Script/MyNetTest.BattlePlayerState|GetPlayerColor _asbattle_player_state) 0))
  (Variables|/Script/MyNetTest.DeathActor|SetColor _returnvalue (Variables|/Script/MyNetTest.BattlePlayerState|GetPlayerColor _asbattle_player_state))
  (Actor|DestroyActor Character)
  (bind _result (Math|Integer|DecrementInt (Variables|Default|GetALifePlayerCount))
    (:%20%20
      (if (== _result 1)
        (CallFunction|DestoryAllTriggerActor)
        (CallFunction|GettheOnlyPlayerAlive)))))

(event EventPlayerPawnHealthIsFull
  (params (Character :type Battle%20Character%20Object%20Reference))
  ;[1 1 1] 有一位玩家血量达到满值，游戏结束
  (CallFunction|DestoryAllTriggerActor)
  (CallFunction|DealwithPlayers Character))

(event EventPostLogin
  (params (NewPlayer :type Player%20Controller%20Object%20Reference))
  (bind _playercontrollerlist (Variables|Default|GetPlayerControllerList))
  ;[1 1 1] PostLogin
  (|CallParentFunction NewPlayer)
  (bind _asbp_battle_player_controller (Utilities|Casting|CastToBP_BattlePlayerController NewPlayer))
  (Utilities|Array|AddUnique _playercontrollerlist _asbp_battle_player_controller)
  (Math|Integer|IncrementInt (Variables|Default|GetALifePlayerCount)
    (:%20%20
      (if (== (Utilities|Array|Length _playercontrollerlist) (Variables|Default|GetMaxPlayerNum))
        (for _array_element (Variables|Default|GetPlayerControllerList)
          (Default|ReadyPlay _array_element))
        (else
          (Default|WaittoStart _asbp_battle_player_controller))))))

(event EventBeginPlay
  (|CallParentFunction)
  (bind _asbp_battle_game_instance (Utilities|Casting|CastToBP_BattleGameInstance (Game|GetGameInstance)))
  (Variables|Default|SetMaxPlayerNum (Variables|/Game/GameSettings/BP_BattleGameInstance.BP_BattleGameInstance_C|GetMaxPlayerNum _asbp_battle_game_instance)))

(fn ConstructionScript)

(fn GettheOnlyPlayerAlive
  (for _array_element (Variables|Default|GetPlayerControllerList)
    (Utilities|IsValid _array_element
      (:Is%20Valid
        (Utilities|IsValid (Pawn|GetControlledPawn _array_element)
          (:Is%20Valid
            (Default|GameWin _array_element))
          (:Is%20Not%20Valid
            (Default|GameLose _array_element)))))))