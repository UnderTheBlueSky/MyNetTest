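; Multiplayer battle character that sets up player info UI and its own player color.
; InitPlayers refreshes player info, has the BP_BattlePlayerController create an info entry for each other player state, then starts per-second health loss.
; It applies the BattlePlayerState color through SetPawnColorOnServer, which relays to SetPawnColorToAll to set a dynamic material parameter on the mesh.
; Key 1 prints the game mode's max player count for debugging.
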(event Custom|InitPlayers
  (bind _playerstate (Variables|Default|GetPlayerState))
  ;[1 1 1] 加载所有玩家的生命值UI显示
  (Class|BattleCharacter|InitPlayersInfo)
  (for _array_element (Variables|Default|GetPlayerStateList)
    (if (not (== _array_element _playerstate))
      (bind _asbp_battle_player_controller (Utilities|Casting|CastToBP_BattlePlayerController (Pawn|GetController)))
      (Default|CreatePlayerInfo _asbp_battle_player_controller _array_element)))
  (bind _asbattle_player_state (Utilities|Casting|CastToBattlePlayerState _playerstate))
  (CallFunction|SetPawnColoronServer (Variables|Character|GetMesh) 0 (Variables|Default|GetMaterialInterface) (Variables|Default|GetParamName) (Variables|/Script/MyNetTest.BattlePlayerState|GetPlayerColor _asbattle_player_state))
  (Class|BattleCharacter|ReducesHealthPerSecond))

(event Custom|SetPawnColorOnServer
  (params (目标 :type Primitive%20Component%20Object%20Reference) (ElementIndex :type Integer) (SourceMaterial :type Material%20Interface%20Object%20Reference) (ParamName :type Name) (Value :type Linear%20Color%20Structure))
  ;[1 1 1] 设置角色颜色
  (CallFunction|SetPawnColortoAll 目标 ElementIndex SourceMaterial ParamName Value))

(event Custom|SetPawnColorToAll
  (params (目标 :type Primitive%20Component%20Object%20Reference) (ElementIndex :type Integer) (SourceMaterial :type Material%20Interface%20Object%20Reference) (ParamName :type Name) (Value :type Linear%20Color%20Structure))
  ;[1 1 1] 设置角色颜色
  (bind _returnvalue (Rendering|Material|CreateDynamicMaterialInstance 目标 ElementIndex SourceMaterial "None" :!class /Script/Engine.PrimitiveComponent))
  (Rendering|Material|SetVectorParameterValue _returnvalue ParamName Value :!class /Script/Engine.MaterialInstanceDynamic))

(event Input|KeyboardEvents|1
  (params (Key :type Key%20Structure :default "None"))
  (:Pressed
    (bind _asbp_battle_game_mode (Utilities|Casting|CastToBP_BattleGameMode (Game|GetGameMode)))
    (Development|PrintString (Utilities|String|ToString(Integer) (Variables|/Script/MyNetTest.BattleGameMode|GetMaxPlayerNum _asbp_battle_game_mode)))))

(fn ConstructionScript)